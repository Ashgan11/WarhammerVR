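; VR test pawn that drives a full-body IK avatar from headset and motion controller tracking.
; Each Tick it writes world transforms of the HDM component and both controllers into the skeletal mesh's Anim_FBIK instance.
; Logic to slide the mesh toward the head after horizontal movement past a threshold exists but never runs, so the graph never repositions the mesh.
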(event EventBeginPlay
  (Variables|Default|SetLastHeadTransform (Transformation|GetWorldTransform (Variables|Default|GetHDM))))

(event EventTick
  (params (DeltaSeconds :type Float%20%28single-precision%29))
  (bind _asanim_fbik (Utilities|Casting|CastToAnim_FBIK (Components|SkeletalMesh|GetAnimInstance (Variables|Default|GetSkeletalMesh))))
  (bind _output_get (Variables|Default|SetCurrentHeadTransform (Transformation|GetWorldTransform (Variables|Default|GetHDM))))
  (Variables|/Game/Testing_Mechanics/FullBody-IK/Blueprints/Anim_FBIK.Anim_FBIK_C|SetIn%20Head%20Transform%20World _asanim_fbik _output_get)
  (Variables|/Game/Testing_Mechanics/FullBody-IK/Blueprints/Anim_FBIK.Anim_FBIK_C|SetIn%20Left%20Hand%20Transform%20World _asanim_fbik (Transformation|GetWorldTransform (Variables|Default|GetMotionController_L)))
  (Variables|/Game/Testing_Mechanics/FullBody-IK/Blueprints/Anim_FBIK.Anim_FBIK_C|SetIn%20Right%20Hand%20Transform%20World _asanim_fbik (Transformation|GetWorldTransform (Variables|Default|GetMotionController_R))))

(fn ConstructionScript)