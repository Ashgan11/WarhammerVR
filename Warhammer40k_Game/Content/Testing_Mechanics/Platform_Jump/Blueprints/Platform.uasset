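; Interactable jump platform that lets a player pawn leap to the platform's end point.
; Interact fires once until Un-Interact resets it, registering the platform as the instigator's interactable and highlighting the mesh through a custom depth stencil.
; Jump spawns a SplineActor from the pawn's location to the EndPoint component and hands the pawn to that actor's Jump to perform the move.
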(event EventInteract
  (params (Instigator :type BP%20Player%20Pawn%20Object%20Reference))
  (Utilities|FlowControl|DoOnce false
    (:Completed
      (Variables|/Game/Testing_Mechanics/Character/Blueprints/BP_PlayerPawn.BP_PlayerPawn_C|SetInteractable Instigator self)
      (Rendering|SetRenderCustomDepth (Variables|Default|GetPlatform) true)
      (Rendering|SetCustomDepthStencilValue (Variables|Default|GetPlatform) (Variables|Default|GetValue)))))

(event EventUn-Interact
  (Utilities|FlowControl|Sequence
    (:then_0
      (Utilities|FlowControl|DoOnce false) ; enters at Reset
    )
    (:then_1
      (Rendering|SetRenderCustomDepth (Variables|Default|GetPlatform) false))))

(event EventJump
  (params (PlayerPawn :type BP%20Player%20Pawn%20Object%20Reference))
  (bind _returnvalue (Transformation|GetActorLocation PlayerPawn))
  (bind _returnvalue_2 (Game|SpawnActorfromClass "/Game/Testing_Mechanics/Platform_Jump/Blueprints/SplineActor.SplineActor_C" (Math|Transform|MakeTransform _returnvalue "0, 0, 0" "1,1,1") "Undefined" self _returnvalue (Transformation|GetWorldLocation (Variables|Default|GetEndPoint)) 0))
  (Default|Jump _returnvalue_2 PlayerPawn))

(fn ConstructionScript)