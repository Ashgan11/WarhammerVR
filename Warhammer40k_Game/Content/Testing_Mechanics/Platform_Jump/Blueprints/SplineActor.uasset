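; Spline-based jump actor that moves a player pawn along an arc between Start and End points.
; Construction builds a three-point spline, raising the apex Height above the higher endpoint and, for long jumps with large height differences, shifting it toward that endpoint.
; Jump fires once via DoOnce, then a timeline scaled to TimeInSec sets the pawn's location each update from constant-velocity, local-space spline samples, without sweeping.
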(event Custom|MovePawn
  (params (Player%20To%20Move :type BP%20Player%20Pawn%20Object%20Reference))
  (bind _time_insec_ (Variables|Default|GetTime%28InSec%29))
  (Components|Timeline|SetPlayRate (Variables|GetDuration) (/ 1.0 _time_insec_))
  (Variables|/Script/Engine.SplineComponent|SetDuration (Variables|Default|GetSpline) _time_insec_)
  (bind _duration (Timeline|Duration PlayFromStart)
    (:Update
      (Transformation|SetActorLocation Player%20To%20Move (Spline|GetLocationatTime (Variables|Default|GetSpline) (* _duration (Variables|Default|GetTime%28InSec%29)) "Local" true) false false))))

(event Custom|Jump
  (params (Player :type BP%20Player%20Pawn%20Object%20Reference))
  (Utilities|FlowControl|DoOnce false
    (:Completed
      (CallFunction|MovePawn Player))))

(fn ConstructionScript
  (CallFunction|GenerateSpline))

(fn GenerateSpline
  (bind _spline (Variables|Default|GetSpline))
  (bind _start (Variables|Default|GetStart))
  (bind _end (Variables|Default|GetEnd))
  (bind _start_2 (Variables|Default|GetStart))
  (bind _end_2 (Variables|Default|GetEnd))
  (bind _start_3 (Variables|Default|GetStart))
  (bind _end_3 (Variables|Default|GetEnd))
  (bind _start_4 (Variables|Default|GetStart))
  (bind _end_4 (Variables|Default|GetEnd))
  (bind _end_5 (Variables|Default|GetEnd))
  (bind _start_5 (Variables|Default|GetStart))
  (bind _type (Variables|Default|GetType))
  (bind _end_6 (Variables|Default|GetEnd))
  (bind _height (Variables|Default|GetHeight))
  (bind _returnvalue (Math|Vector|GetUnitDirection(Vector) (Math|Vector|MakeVector (.x _end_2) (.y _end_2) 0.0) (Math|Vector|MakeVector (.x _start_2) (.y _start_2) 0.0)))
  (bind _returnvalue_2 (Math|Vector|Distance2D(Vector) (Math|Vector2D|MakeVector2D (.x _start) (.y _start)) (Math|Vector2D|MakeVector2D (.x _end) (.y _end))))
  (bind _returnvalue_3 (Math|Vector|GetUnitDirection(Vector) (Math|Vector|MakeVector (.x _start_3) (.y _start_3) 0.0) (Math|Vector|MakeVector (.x _end_3) (.y _end_3) 0.0)))
  (bind _returnvalue_4 (Math|Vector|GetUnitDirection(Vector) (Math|Vector|MakeVector (.x _start_4) (.y _start_4) 0.0) (Math|Vector|MakeVector (.x _end_4) (.y _end_4) 0.0)))
  (bind _returnvalue_5 (+ (.z _end_6) _height))
  (bind _distance (Utilities|GetDistance (.z _start) (.z _end)))
  (bind _returnvalue_6 (/ _returnvalue_2 2.0))
  (bind _returnvalue_7 (Math|Float|Clamp(Float) _distance 5e+01 1e+03))
  (bind _returnvalue_8 (- _returnvalue_6 1e+03))
  (bind _returnvalue_9 (/ _returnvalue_7 1e+03))
  (bind _returnvalue_10 (- 1.0 _returnvalue_9))
  (bind _returnvalue_11 (* _returnvalue_8 _returnvalue_10))
  (bind _returnvalue_12 (+ 1e+03 _returnvalue_11))
  (bind _returnvalue_13 (+ 1e+03 _returnvalue_11))
  (if (or (> 2e+03 _returnvalue_2) (< _distance 5e+01))
    (LocalVariables|SetXYMiddle (Math|Vector2D|MakeVector2D (* (.x _returnvalue_3) _returnvalue_6) (* (.y _returnvalue_3) _returnvalue_6)))
    (elif (> (.z (Variables|Default|GetStart)) (.z (Variables|Default|GetEnd)))
      (LocalVariables|SetXYMiddle (Math|Vector2D|MakeVector2D (+ (* (.x _returnvalue_4) _returnvalue_12) (.x _start_5)) (+ (* (.y _returnvalue_4) _returnvalue_12) (.y _start_5))))
      (else
        (LocalVariables|SetXYMiddle (Math|Vector2D|MakeVector2D (+ (* (.x _returnvalue) _returnvalue_13) (.x _end_5)) (+ (* (.y _returnvalue) _returnvalue_13) (.y _end_5)))))))
  (Math|Float|CompareFloat (.z (Variables|Default|GetStart)) (.z (Variables|Default|GetEnd))
    (:>
      (Variables|Default|SetMiddle (Math|Vector|MakeVector (.x (LocalVariables|GetXYMiddle)) (.y (LocalVariables|GetXYMiddle)) (+ (.z (Variables|Default|GetStart)) _height))))
    (:==
      (Variables|Default|SetMiddle (Math|Vector|MakeVector (.x (LocalVariables|GetXYMiddle)) (.y (LocalVariables|GetXYMiddle)) _returnvalue_5)))
    (:<
      (Variables|Default|SetMiddle (Math|Vector|MakeVector (.x (LocalVariables|GetXYMiddle)) (.y (LocalVariables|GetXYMiddle)) _returnvalue_5))))
  (Spline|ClearSplinePoints _spline true)
  (Spline|AddSplinePoint _spline (Variables|Default|GetStart) "Local" true)
  (Spline|AddSplinePoint _spline (Variables|Default|GetMiddle) "Local" true)
  (Spline|AddSplinePoint _spline (Variables|Default|GetEnd) "Local" true)
  (Spline|SetSplinePointType _spline 0 _type true)
  (Spline|SetSplinePointType _spline 1 _type true)
  (Spline|SetSplinePointType _spline 2 _type true))