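; Test game mode for the in-game menu prototype, handling quitting, pausing and session start and end.
; Session events open the test in-game and main menu levels by name.
; PauseGame alternates between spawning and destroying a 3D pause menu actor, without pausing the game itself.
; GetPauseWidgetPosition supplies the spawn transform, but its pawn-facing offset math is unconnected and omits the pawn's location.
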(event EventQuitGame
  (Game|QuitGame (Game|GetPlayerController 0) "Quit" false))

(event EventStartSession
  (Game|OpenLevel(byName) "TestInGameMenu"))

(event EventQuitSession
  (Game|OpenLevel(byName) "TestMainMenu"))

(event EventPauseGame
  (Utilities|FlowControl|FlipFlop
    (:A
      (bind _returnvalue (Game|SpawnActorfromClass "/Game/Testing_Mechanics/In-Game_Menu/Blueprints/BP_PauseMenu3D.BP_PauseMenu3D_C" (Utilities|GetPauseWidgetPosition) "Undefined" 0 0))
      (Variables|Default|SetPauseWidget _returnvalue))
    (:B
      (Actor|DestroyActor (Variables|Default|GetPauseWidget)))))

(fn ConstructionScript)