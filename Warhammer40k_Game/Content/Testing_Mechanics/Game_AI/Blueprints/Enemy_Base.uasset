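; Base enemy character that chases the player, takes damage with knockback, and explodes when destroyed.
; BeginPlay fills health and sets the player pawn as its SimpleAIController's move target.
; Damage types convert hits into damage and force: AnyDamage reduces health, destroying the actor at zero, while Point and Radial damage launch it with an upward-biased impulse.
; Point hits use the hit normal as knockback origin, and Lightness affects only the debug print.
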(event Custom|Spawn%20Emitter
  (params (EmitterTemplate :type Particle%20System%20Object%20Reference))
  (bind _returnvalue (Transformation|GetActorTransform))
  ;[1 1 1] Death Event
  (Effects|SpawnEmitteratLocation EmitterTemplate (.location _returnvalue) (.rotation _returnvalue) (.scale _returnvalue)))

(event EventBeginPlay
  (Variables|Values|SetCurrentHealth (Variables|Values|GetMaxHealth))
  ;[1 1 1] Possibly placeholder if we add a more complex behavior tree later.
  (bind _assimple_aicontroller (Utilities|Casting|CastToSimpleAIController (AI|GetAIController 0)))
  (Variables|/Game/Testing_Mechanics/Game_AI/Blueprints/SimpleAIController.SimpleAIController_C|SetMoveTarget _assimple_aicontroller (Game|Player|GetPlayerPawn 0)))

(event Game|Damage|EventPointDamage
  (params (Damage :type Float%20%28single-precision%29) (DamageType :type Damage%20Type%20Object%20Reference) (HitLocation :type Vector :default "0, 0, 0") (HitNormal :type Vector :default "0, 0, 0") (HitComponent :type Primitive%20Component%20Object%20Reference) (BoneName :type Name :default "None") (ShotFromDirection :type Vector :default "0, 0, 0") (InstigatedBy :type Controller%20Object%20Reference) (DamageCauser :type Actor%20Object%20Reference) (HitInfo :type Hit%20Result%20Structure%20%28by%20ref%29))
  ;[1 1 1] Damage Responses
  (bind _force (Class|DamageTypeInterface|GetDamageandForce(Message) DamageType Damage))
  (CallFunction|ApplyKnockback _force HitNormal))

(event Game|Damage|EventRadialDamage
  (params (DamageReceived :type Float%20%28single-precision%29) (DamageType :type Damage%20Type%20Object%20Reference) (Origin :type Vector :default "0, 0, 0") (HitInfo :type Hit%20Result%20Structure%20%28by%20ref%29) (InstigatedBy :type Controller%20Object%20Reference) (DamageCauser :type Actor%20Object%20Reference))
  ;[1 1 1] Damage Responses
  (bind _force (Class|DamageTypeInterface|GetDamageandForce(Message) DamageType DamageReceived))
  (CallFunction|ApplyKnockback _force Origin))

(event Game|Damage|EventAnyDamage
  (params (Damage :type Float%20%28single-precision%29) (DamageType :type Damage%20Type%20Object%20Reference) (InstigatedBy :type Controller%20Object%20Reference) (DamageCauser :type Actor%20Object%20Reference))
  ;[1 1 1] Damage Responses
  (bind _damage (Class|DamageTypeInterface|GetDamageandForce(Message) DamageType Damage))
  (CallFunction|TakeDamage _damage))

(event EventDestroyed
  ;[1 1 1] Death Event
  (CallFunction|SpawnEmitter "/Game/StarterContent/Particles/P_Explosion.P_Explosion"))

(fn ConstructionScript)

(fn ApplyKnockback
  (params (Force :type Float%20%28single-precision%29) (Origin :type Vector))
  (Development|PrintString (Utilities|String|Append "Force applied: " (Utilities|String|ToString(Float) (* Force (Variables|Values|GetLightness))) " from position: " (Utilities|String|ToString(Vector) Origin)) true true "(R=0.000000,G=0.660000,B=1.000000,A=1.000000)" 5.0)
  (Components|Movement|StopMovementImmediately (Variables|Character|GetCharacterMovement))
  (Physics|AddImpulse (Variables|Character|GetCharacterMovement) (+ (* (Math|Vector|GetUnitDirection(Vector) Origin (Transformation|GetActorLocation)) Force) (* (Math|Vector|VectorUp) (* 0.34 Force))) true))

(fn TakeDamage
  (params (Damage :type Float%20%28single-precision%29))
  (bind _output_get (Variables|Values|SetCurrentHealth (Math|Float|Clamp(Float) (- (Variables|Values|GetCurrentHealth) Damage) 0.0 (Variables|Values|GetMaxHealth))))
  (Development|PrintString (Utilities|String|ToString(Float) _output_get) true true "(R=0.000000,G=0.660000,B=1.000000,A=1.000000)" 5.0)
  (Math|Float|CompareFloat (Variables|Values|GetCurrentHealth) 0.0
    (:==
      (Actor|DestroyActor))))