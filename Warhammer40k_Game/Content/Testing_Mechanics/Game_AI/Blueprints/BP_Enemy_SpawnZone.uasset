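; Enemy spawn zone actor that spawns AI pawns of a given class at random points within a box area.
; The construction script sizes the SpawnArea box from SpawnAreaExtent's X and Y, with a fixed shallow height.
; SpawnEnemyAtRandomPoint passes a random world-axis-aligned point from GetRandomPoint to SpawnAIFromClass.
; The event graph is empty, so spawning relies on external calls.
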(event EventBeginPlay)

(event Collision|EventActorBeginOverlap
  (params (OtherActor :type Actor%20Object%20Reference)))

(event EventTick
  (params (DeltaSeconds :type Float%20%28single-precision%29)))

(fn ConstructionScript
  (bind _spawn_area_extent (Variables|Default|GetSpawn%20Area%20Extent))
  (bind (_x _y) (Math|Vector2D|BreakVector2D _spawn_area_extent))
  (Components|Box|SetBoxExtent (Variables|Default|GetSpawnArea) (Math|Vector|MakeVector _x _y 2e+01) true))

(fn GetRandomPoint
  (bind _spawnarea (Variables|Default|GetSpawnArea))
  (return (Math|Random|RandomPointinBoundingBox (Transformation|GetWorldLocation _spawnarea) (Variables|/Script/Engine.BoxComponent|GetBoxExtent _spawnarea))))

(fn SpawnEnemyatRandomPoint
  (params (PawnClass :type Pawn%20Class%20Reference))
  (bind _randompoint (CallFunction|GetRandomPoint))
  (AI|SpawnAIFromClass PawnClass 0 _randompoint "0, 0, 0" false 0))