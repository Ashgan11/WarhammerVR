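; Base enemy character that handles health, melee attacks, knockback and an explosion effect when destroyed.
; Attacks are picked at random from AttackList, with montage notifies pausing and resuming a looping timer that capsule-traces at a socket.
; DamagePlayer skips actors already in HitActors until EndHitBox clears it.
; Damage types supply damage and force for incoming hits, with point and radial knockback cancelling the current attack montage.
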(event Custom|Spawn%20Emitter
  (params (EmitterTemplate :type Particle%20System%20Object%20Reference))
  (bind _returnvalue (Transformation|GetActorTransform))
  ;[1 1 1] Death Event
  (Effects|SpawnEmitteratLocation EmitterTemplate (.location _returnvalue) (.rotation _returnvalue) (.scale _returnvalue)))

(event Custom|StartAttack
  ;[1 1 1] Ghetto way of telling the animation BP to please start attacking.
  (Variables|Default|SetattackNotifier true))

(event Custom|BeginHitBox
  (params (Hitbox%20Component :type Primitive%20Component%20Object%20Reference))
  ;[1 1 1] Enable / Disable any target hitbox component.
  (Collision|SetCollisionEnabled Hitbox%20Component "QueryOnly"))

(event Custom|EndHitBox
  (params (Hitbox%20Component :type Primitive%20Component%20Object%20Reference))
  ;[1 1 1] Enable / Disable any target hitbox component.
  (Utilities|Array|Clear (Variables|Default|GetHitActors))
  (Collision|SetCollisionEnabled Hitbox%20Component "NoCollision")
  (Variables|Default|SetattackNotifier false))

(event Custom|Begin%20Attack
  (params (Executing%20Attack :type S%20Attack%20Structure))
  (bind _hittracetimer (Variables|Default|GetHitTraceTimer))
  ;[1 1 1] Logic to initiate an attack with a given SAttack struct's parameters.
  (bind _output_get (Variables|Default|SetCurrentAttack Executing%20Attack))
  (bind _notifyname (Animation|Montage|PlayMontage (Variables|Character|GetMesh) (.Animation (Utilities|Struct|BreakSAttack _output_get)))
    (:OnCompleted
      (CallFunction|FinishAttack))
    (:OnInterrupted
      (CallFunction|InterruptAttack))
    (:OnNotifyBegin
      (switch name _notifyname
        (:BeginDamage
          (Utilities|Time|UnpauseTimerbyHandle _hittracetimer))
        (:EndDamage
          (Utilities|Time|PauseTimerbyHandle _hittracetimer))))))

(event Custom|Select%20Attack
  ;[1 1 1] Simple random logic - should be overridable on children!
  (if (not (AI|Components|NavMovement|IsFalling (Variables|Character|GetCharacterMovement)))
    (CallFunction|BeginAttack (.OutItem (Utilities|Array|Random (Variables|Gameplay|GetAttackList))))))

(event Custom|Finish%20Attack
  ;[1 1 1] Placeholder events if we want to do stuff when finishing or interrupting an attack
)

(event Custom|Interrupt%20Attack
  ;[1 1 1] Placeholder events if we want to do stuff when finishing or interrupting an attack
  (Utilities|Time|PauseTimerbyHandle (Variables|Default|GetHitTraceTimer)))

(event Custom|HitTrace
  (bind _mesh (Variables|Character|GetMesh))
  (bind _currentattack (Variables|Default|GetCurrentAttack))
  (bind _currentattack_2 (Variables|Default|GetCurrentAttack))
  (bind (_attackname _damage _damagetype) (Utilities|Struct|BreakSAttack _currentattack_2))
  (bind (_attackname_2 _damage_2 _damagetype_2 _animation _hitcapsule_socket _hitcapsule_radius _hitcapsule_halfheight) (Utilities|Struct|BreakSAttack _currentattack))
  (bind _returnvalue (Transformation|GetSocketLocation _mesh _hitcapsule_socket))
  ;[1 1 1] Traces a hit capsule during attacks.
  (bind (_outhit _returnvalue_2) (Collision|CapsuleTraceByChannel _returnvalue _returnvalue _hitcapsule_radius _hitcapsule_halfheight "TraceTypeQuery2" false (Utilities|Array|MakeArray 0) "ForDuration"))
  (if _returnvalue_2
    ;;[1 1 1] Check if attack was blocked here??
    (if true
      (CallFunction|DamagePlayer (.HitActor (Collision|BreakHitResult _outhit)) _damage _damagetype))))

(event EventBeginPlay
  ;[1 1 1] Initialize CurrentHealth
  (Variables|Gameplay|SetCurrentHealth (Variables|Gameplay|GetMaxHealth))
  (bind _returnvalue (Utilities|Time|SetTimerbyEvent (delegate Custom|HitTrace) (Variables|Gameplay|GetHitTraceInterval) true))
  (bind _output_get (Variables|Default|SetHitTraceTimer _returnvalue))
  (Utilities|Time|PauseTimerbyHandle _output_get))

(event Game|Damage|EventPointDamage
  (params (Damage :type Float%20%28single-precision%29) (DamageType :type Damage%20Type%20Object%20Reference) (HitLocation :type Vector :default "0, 0, 0") (HitNormal :type Vector :default "0, 0, 0") (HitComponent :type Primitive%20Component%20Object%20Reference) (BoneName :type Name :default "None") (ShotFromDirection :type Vector :default "0, 0, 0") (InstigatedBy :type Controller%20Object%20Reference) (DamageCauser :type Actor%20Object%20Reference) (HitInfo :type Hit%20Result%20Structure%20%28by%20ref%29))
  ;[1 1 1] Damage Responses
  (bind _force (Class|BPIDamageTypeInterface|GetDamageandForce(Message) DamageType Damage))
  (CallFunction|ApplyKnockback _force HitNormal))

(event Game|Damage|EventRadialDamage
  (params (DamageReceived :type Float%20%28single-precision%29) (DamageType :type Damage%20Type%20Object%20Reference) (Origin :type Vector :default "0, 0, 0") (HitInfo :type Hit%20Result%20Structure%20%28by%20ref%29) (InstigatedBy :type Controller%20Object%20Reference) (DamageCauser :type Actor%20Object%20Reference))
  ;[1 1 1] Damage Responses
  (bind _force (Class|BPIDamageTypeInterface|GetDamageandForce(Message) DamageType DamageReceived))
  (CallFunction|ApplyKnockback _force Origin))

(event Game|Damage|EventAnyDamage
  (params (Damage :type Float%20%28single-precision%29) (DamageType :type Damage%20Type%20Object%20Reference) (InstigatedBy :type Controller%20Object%20Reference) (DamageCauser :type Actor%20Object%20Reference))
  ;[1 1 1] Damage Responses
  (bind _damage (Class|BPIDamageTypeInterface|GetDamageandForce(Message) DamageType Damage))
  (CallFunction|TakeDamage _damage))

(event EventDestroyed
  ;[1 1 1] Death Event
  (CallFunction|SpawnEmitter "/Game/StarterContent/Particles/P_Explosion.P_Explosion"))

(fn ConstructionScript)

(fn ApplyKnockback
  (params (Force :type Float%20%28single-precision%29) (Origin :type Vector))
  (Components|Movement|StopMovementImmediately (Variables|Character|GetCharacterMovement))
  (Physics|AddImpulse (Variables|Character|GetCharacterMovement) (+ (* (Math|Vector|GetUnitDirection(Vector) Origin (Transformation|GetActorLocation)) Force) (* (Math|Vector|VectorUp) (* 0.34 Force))) true)
  ;[1 1 1] Cancel attack if in progress
  (Animation|StopAnimMontage (.Animation (Utilities|Struct|BreakSAttack (Variables|Default|GetCurrentAttack)))))

(fn TakeDamage
  (params (Damage :type Float%20%28single-precision%29))
  (Variables|Gameplay|SetCurrentHealth (Math|Float|Clamp(Float) (- (Variables|Gameplay|GetCurrentHealth) Damage) 0.0 (Variables|Gameplay|GetMaxHealth)))
  (Math|Float|CompareFloat (Variables|Gameplay|GetCurrentHealth) 0.0
    (:==
      (Actor|DestroyActor))))

(fn DamagePlayer
  (params (Other%20Actor :type Actor%20Object%20Reference) (BaseDamage :type Float%20%28single-precision%29) (DamageTypeClass :type Damage%20Type%20Class%20Reference))
  (if (== Other%20Actor self)
    _
    (elif (and (not (Utilities|Array|ContainsItem (Variables|Default|GetHitActors) Other%20Actor)) (!= (Utilities|GetClass Other%20Actor) "BP_Enemy_Base_C"))
      (bind _returnvalue (Game|Damage|ApplyDamage Other%20Actor BaseDamage 0 self DamageTypeClass))
      (Utilities|Array|Add (Variables|Default|GetHitActors) Other%20Actor)
      (return _returnvalue)
      (else
        _)))
  (return -1.0))