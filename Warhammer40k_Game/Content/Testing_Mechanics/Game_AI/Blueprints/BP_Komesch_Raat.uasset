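; BP_Komesch_Raat is a test game-AI Blueprint with a modular skeletal body that reacts to hits per bone.
; The construction script adds a component per mapped mesh part, slaved to the main Mesh via master pose and copying its materials, with random selection switched off.
; Mesh hits look up the struck bone's component, give it a random material from MaterialList, and print "Headshot" for the Head.
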(event OnComponentHit(Mesh)
  (params (HitComponent :type Primitive%20Component%20Object%20Reference) (OtherActor :type Actor%20Object%20Reference) (OtherComp :type Primitive%20Component%20Object%20Reference) (NormalImpulse :type Vector :default "0, 0, 0") (Hit :type Hit%20Result%20Structure%20%28by%20ref%29))
  (bind _skeletalmeshcompmap (Variables|Default|GetSkeletalMeshCompMap))
  (bind (_value _returnvalue) (Utilities|Map|Find _skeletalmeshcompmap (.hitbonename Hit)))
  (if _returnvalue
    (switch name (.hitbonename Hit)
      (:Default
        _)
      (:head
        (Development|PrintString "Headshot")))
    (Rendering|Material|SetMaterial _value 0 (.OutItem (Utilities|Array|Random (Variables|Default|GetMaterialList))))))

(event EventBeginPlay
  (|CallParentFunction) ; This node is disabled and will not be called.\nDrag off pins to build functionality.
)

(event Collision|EventActorBeginOverlap
  (params (OtherActor :type Actor%20Object%20Reference)))

(event EventTick
  (params (DeltaSeconds :type Float%20%28single-precision%29)))

(fn ConstructionScript
  (bind _mesh (Variables|Character|GetMesh))
  ;[0.498 0 1] MODULAR BODY CONSTRUCTION
  (if (not (Variables|Default|GetbHasSkeletalComponents))
    (bind _values (Utilities|Map|Values (Variables|Default|GetSkeletalMeshPartsMap)))
    (for _array_element _values
      (bind _returnvalue (AddComponent|AddSkeletalMeshComponent true))
      (Utilities|Array|Add (Variables|Default|GetSkeletalMeshComponentList) _returnvalue)
      (Class|SkinnedMeshComponent|SetSkeletalMesh _returnvalue _array_element true)
      (Transformation|AttachComponentToComponent _returnvalue _mesh "None" "KeepRelative" "KeepRelative" "KeepRelative" true)
      (Class|SkinnedMeshComponent|SetMasterPoseComponent _returnvalue _mesh false)
      (for (_array_element_2 _array_index) (Rendering|Material|GetMaterials _mesh)
        (bind _materialout (|IsRandom_2 _array_element_2 false))
        (Rendering|Material|SetMaterial _returnvalue _array_index _materialout)))
    (Variables|Default|SetbHasSkeletalComponents true)))