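; CaptureZone is a platform-capture test actor: a zone scaled by construction-script variables that tracks capture progress over time.
; Two looping timers, created paused, drive Capturing, which raises load time until it sets Captured, and Escape, which drains it to zero.
; Overlap events only check Captured; the cast and timer-switching logic is disconnected, so neither timer gets unpaused.
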(event OnComponentBeginOverlap(OverlapZone)
  (params (OverlappedComponent :type Primitive%20Component%20Object%20Reference) (OtherActor :type Actor%20Object%20Reference) (OtherComp :type Primitive%20Component%20Object%20Reference) (OtherBodyIndex :type Integer) (bFromSweep :type Boolean) (SweepResult :type Hit%20Result%20Structure%20%28by%20ref%29))
  (if (Variables|GameplayVar|GetCaptured)
    _))

(event OnComponentEndOverlap(OverlapZone)
  (params (OverlappedComponent :type Primitive%20Component%20Object%20Reference) (OtherActor :type Actor%20Object%20Reference) (OtherComp :type Primitive%20Component%20Object%20Reference) (OtherBodyIndex :type Integer))
  (if (Variables|GameplayVar|GetCaptured)
    _))

(event EventBeginPlay
  (bind _returnvalue (Utilities|Time|SetTimerbyFunctionName 0 "Capturing" 0.1 true))
  (bind _output_get (Variables|Timers|SetCapturing_Timer _returnvalue))
  (Utilities|Time|PauseTimerbyHandle _output_get)
  (bind _returnvalue_2 (Utilities|Time|SetTimerbyFunctionName 0 "Escape" 0.1 true))
  (bind _output_get_2 (Variables|Timers|SetEscape_Timer _returnvalue_2))
  (Utilities|Time|PauseTimerbyHandle _output_get_2))

(fn ConstructionScript
  (bind _zone_scale (Variables|Construct|GetZone_Scale))
  (Transformation|SetWorldScale3D (Variables|Default|GetZone) (Math|Vector|MakeVector _zone_scale _zone_scale (Variables|Construct|GetZone_Height))))

(fn Capturing
  (bind _output_get (Variables|GameplayVar|SetCurrent_LoadTime (+ (Variables|GameplayVar|GetCurrent_LoadTime) 0.1)))
  (if (>= _output_get (Variables|GameplayVar|GetMax_LoadTime))
    (Variables|GameplayVar|SetCaptured true)
    (Utilities|Time|PauseTimerbyHandle (Variables|Timers|GetCapturing_Timer)))
  (return))

(fn Escape
  (bind _output_get (Variables|GameplayVar|SetCurrent_LoadTime (- (Variables|GameplayVar|GetCurrent_LoadTime) 0.1)))
  (if (<= _output_get 0.0)
    (Utilities|Time|PauseTimerbyHandle (Variables|Timers|GetEscape_Timer)))
  (return))