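; BP_PlayerPawn is a player pawn with left and right motion controllers and a configurable weapon slot for each side.
; Its construction script checks each side's weapon class and, when valid, hides that controller's device model and assigns the class to that side's child actor component.
; The event graph holds no active logic.
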(event EventBeginPlay)

(fn ConstructionScript
  (Utilities|FlowControl|Sequence
    (:then_0
      (if (Utilities|IsValidClass (Variables|Default|GetWeaponClass_Left))
        (Variables|/Script/HeadMountedDisplay.MotionControllerComponent|SetbDisplayDeviceModel (Variables|Default|GetMotionControllerLeft) false)
        (ChildActorComponent|SetChildActorClass (Variables|Default|GetWeaponLeft) (Variables|Default|GetWeaponClass_Left))))
    (:then_1
      (if (Utilities|IsValidClass (Variables|Default|GetWeaponClass_Right))
        (Variables|/Script/HeadMountedDisplay.MotionControllerComponent|SetbDisplayDeviceModel (Variables|Default|GetMotionControllerRight) false)
        (ChildActorComponent|SetChildActorClass (Variables|Default|GetWeaponRight) (Variables|Default|GetWeaponClass_Right))))))