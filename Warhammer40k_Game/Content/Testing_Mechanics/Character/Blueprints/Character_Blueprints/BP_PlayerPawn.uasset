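; VR player pawn with two motion-controller weapons and view-directed platform interaction.
; With an HMD enabled, BeginPlay sets eye-level tracking and creates a looping platform-trace timer, immediately paused.
; The trace sends interact messages to hit actors, with a DoOnce limiting un-interact to one call per miss streak.
; Construction fills weapon child-actor slots from configurable classes, hiding controller models; trigger inputs are forwarded to each weapon as messages.
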(event Custom|LineTraceToPlatform
  (bind _arrow_viewdir (Variables|Default|GetArrow_ViewDir))
  ;[1 1 1] Platform Trace & Interact
  (bind (_outhit _returnvalue) (Collision|LineTraceByChannel (Transformation|GetWorldLocation _arrow_viewdir) (* (Math|Vector|GetForwardVector _arrow_viewdir) (Variables|Default|GetPlatformTraceLength)) "TraceTypeQuery1" false 0 "None"))
  (if _returnvalue
    (Utilities|FlowControl|Sequence
      (:then_0
        (CallFunction|ResetUn-Interact))
      (:then_1
        (Class|BPIPlatform|Interact(Message) (.HitActor (Collision|BreakHitResult _outhit)) self)))
    (else
      (Utilities|FlowControl|DoOnce true
        (:Completed
          (Class|BPIPlatform|Un-Interact(Message) (Variables|Default|GetInteractable))
          (Variables|Default|SetInteractable 0))))))

(event Custom|Reset%20Un-Interact
  ;[1 1 1] Platform Trace & Interact
  (Utilities|FlowControl|DoOnce true) ; enters at Reset
)

(event EventBeginPlay
  ;[1 1 1] Init
  (if (Class|HeadMountedDisplayFunctionLibrary|IsHeadMountedDisplayEnabled)
    (Class|HeadMountedDisplayFunctionLibrary|SetTrackingOrigin "Eye")
    (bind _returnvalue (Utilities|Time|SetTimerbyEvent (delegate Custom|LineTraceToPlatform) 0.1 true))
    (Utilities|Time|PauseTimerbyHandle _returnvalue)))

(event Input|ActionEvents|InputActionTriggerLeft
  (params (Key :type Key%20Structure))
  (bind _weaponleft (Variables|Default|GetWeaponLeft))
  ;[1 1 1] Trigger Inputs
  (:Pressed
    (Class|BPIWeapon|InputTriggerPressed(Message) _weaponleft))
  (:Released
    (Class|BPIWeapon|InputTriggerRelease(Message) _weaponleft)))

(event Input|ActionEvents|InputActionTriggerRight
  (params (Key :type Key%20Structure))
  (bind _weaponright (Variables|Default|GetWeaponRight))
  ;[1 1 1] Trigger Inputs
  (:Pressed
    (Class|BPIWeapon|InputTriggerPressed(Message) _weaponright))
  (:Released
    (Class|BPIWeapon|InputTriggerRelease(Message) _weaponright)))

(fn ConstructionScript
  (Utilities|FlowControl|Sequence
    (:then_0
      (if (Utilities|IsValidClass (Variables|Default|GetWeaponClass_Left))
        (Variables|/Script/HeadMountedDisplay.MotionControllerComponent|SetbDisplayDeviceModel (Variables|Default|GetMotionControllerLeft) false)
        (ChildActorComponent|SetChildActorClass (Variables|Default|GetWeaponLeft) (Variables|Default|GetWeaponClass_Left))))
    (:then_1
      (if (Utilities|IsValidClass (Variables|Default|GetWeaponClass_Right))
        (Variables|/Script/HeadMountedDisplay.MotionControllerComponent|SetbDisplayDeviceModel (Variables|Default|GetMotionControllerRight) false)
        (ChildActorComponent|SetChildActorClass (Variables|Default|GetWeaponRight) (Variables|Default|GetWeaponClass_Right))))))