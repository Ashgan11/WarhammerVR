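; Ranged weapon actor that fires projectiles for its parent Pawn in Semi-Auto, Full-Auto or Charge-Up mode, drawing on an ammo pool.
; Tick and trigger press/release dispatch by fire mode to cooldown-gated shots, a looping fire timer paused and unpaused by the trigger, or charge buildup.
; Charged releases spawn a separate projectile with charge-scaled damage, falling back to a normal shot when charge or ammo is too low.
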(event Custom|RefillAmmo
  (params (Bonus%20Ammo :type Float%20%28single-precision%29))
  ;[1 1 1] Gain & Lose Ammo Events
  (Variables|Gameplay|SetAmmunitionCur (Math|Float|Clamp(Float) (+ Bonus%20Ammo (Variables|Gameplay|GetAmmunitionCur)) (Variables|Gameplay|GetAmmunitionCur) (Variables|Gameplay|GetAmmunitionMax))))

(event Custom|Shoot
  ;[1 1 1] Shoot Projectile
  (Math|Float|CompareFloat (Variables|Gameplay|GetAmmunitionCur) (Variables|Gameplay|GetAmmunitionCost)
    (:>
      (bind _aspawn (Utilities|Casting|CastToPawn (Actor|GetParentActor) :!label _label)
        (:then
          (Game|SpawnActorfromClass (Variables|Gameplay|GetProjectileClass) (Transformation|GetWorldTransform (Variables|Default|GetArrow_ProjectileSpawn)) "Undefined" _aspawn (Variables|Default|GetDamageType) (Variables|Default|GetDamageAmount) _aspawn)
          (CallFunction|ReduceAmmo (Variables|Gameplay|GetAmmunitionCost)))
        (:CastFailed
          (Development|PrintString "Bad parent actor!"))))
    (:==
      (goto _label))
    (:<
      (Development|PrintString "Out of ammo!"))))

(event Custom|Pressed_Charge
  ;[1 1 1] Trigger Events
  (Variables|Internal|SetCharge_ShotCharge 0.0))

(event Custom|Release_Charge
  ;[1 1 1] Trigger Events
  (Math|Float|CompareFloat (Variables|Gameplay|GetAmmunitionCur) (Variables|Gameplay-Charge|GetCharge_ChargeAmmunitionCost)
    (:>
      (Math|Float|CompareFloat (Variables|Internal|GetCharge_ShotCharge) (Variables|Gameplay-Charge|GetCharge_MinTimeToBeginCharge) :!label _label
        (:>
          (CallFunction|ChargeShot :!label _label_2))
        (:==
          (goto _label_2))
        (:<
          (CallFunction|Shoot)))
      (Variables|Internal|SetCharge_ShotCharge 0.0))
    (:==
      (goto _label))
    (:<
      (CallFunction|Shoot))))

(event Custom|Tick_Charge
  ;[1 1 1] Tick Events
  (bind _charge_percent (CallFunction|GetChargePercent))
  (Variables|Internal|SetChargePercent _charge_percent)
  (if (Variables|Internal|GetIsInputTriggerPressed?)
    (Variables|Internal|SetCharge_ShotCharge (Math|Float|Clamp(Float) (+ (Utilities|Time|GetWorldDeltaSeconds) (Variables|Internal|GetCharge_ShotCharge)) 0.0 (Variables|Gameplay-Charge|GetCharge_FullChargeTime)))))

(event Custom|ChargeShot
  ;[1 1 1] Charge Shot
  (bind _aspawn (Utilities|Casting|CastToPawn (Actor|GetParentActor)))
  (Game|SpawnActorfromClass (Variables|Gameplay-Charge|GetCharge_ProjectileClass) (Transformation|GetWorldTransform (Variables|Default|GetArrow_ProjectileSpawn)) "Undefined" _aspawn (Variables|Gameplay-Charge|GetCharge_DamageType) (Math|Float|Clamp(Float) (* (/ (Variables|Internal|GetCharge_ShotCharge) (Variables|Gameplay-Charge|GetCharge_FullChargeTime)) (Variables|Gameplay-Charge|GetCharge_FullChargeDamage)) (Variables|Default|GetDamageAmount) (Variables|Gameplay-Charge|GetCharge_FullChargeDamage)) _aspawn)
  (CallFunction|ReduceAmmo (Variables|Gameplay-Charge|GetCharge_ChargeAmmunitionCost)))

(event Custom|ReduceAmmo
  (params (Lost%20Ammo :type Float%20%28single-precision%29))
  ;[1 1 1] Gain & Lose Ammo Events
  (Variables|Gameplay|SetAmmunitionCur (Math|Float|Clamp(Float) (- (Variables|Gameplay|GetAmmunitionCur) Lost%20Ammo) 0.0 (Variables|Gameplay|GetAmmunitionMax))))

(event Custom|Automatic%20Shoot
  ;[1 1 1] Set up periodic function for automatic fire. Only relevant if weapon uses full-auto.
  (CallFunction|Shoot))

(event Custom|Tick_Semi%20Auto
  ;[1 1 1] Tick Events
  (Variables|Gameplay-Semi-Auto|SetSemiAuto_FireCooldown (Math|Float|Clamp(Float) (+ (Utilities|Time|GetWorldDeltaSeconds) (Variables|Internal|GetSemiAuto_FireCooldownCur)) 0.0 (Variables|Gameplay-Semi-Auto|GetSemiAuto_FireCooldown))))

(event Custom|Tick_Full%20Auto
  ;[1 1 1] Tick Events
)

(event Custom|Pressed_Semi%20Auto
  ;[1 1 1] Trigger Events
  (Math|Float|CompareFloat (Variables|Internal|GetSemiAuto_FireCooldownCur) (Variables|Gameplay-Semi-Auto|GetSemiAuto_FireCooldown)
    (:>
      _)
    (:==
      _))
  (CallFunction|Shoot)
  (Variables|Internal|SetSemiAuto_FireCooldownCur 0.0))

(event Custom|Release_Semi%20Auto
  ;[1 1 1] Trigger Events
)

(event Custom|Pressed_Full%20Auto
  ;[1 1 1] Trigger Events
  (Utilities|Time|UnpauseTimerbyHandle (Variables|Internal|GetFullAuto_AutomaticShootHandle)))

(event Custom|Release_Full%20Auto
  ;[1 1 1] Trigger Events
  (Utilities|Time|PauseTimerbyHandle (Variables|Internal|GetFullAuto_AutomaticShootHandle)))

(event EventBeginPlay
  ;[1 1 1] Initialize current ammo
  (Variables|Gameplay|SetAmmunitionCur (Variables|Gameplay|GetAmmunitionMax))
  ;[1 1 1] Set up periodic function for automatic fire. Only relevant if weapon uses full-auto.
  (bind _returnvalue (Utilities|Time|SetTimerbyEvent (delegate Custom|Automatic%20Shoot) (Variables|Gameplay-Full-Auto|GetFullAuto_FireRate) true))
  (bind _output_get (Variables|Internal|SetFullAuto_AutomaticShootHandle _returnvalue))
  (Utilities|Time|PauseTimerbyHandle _output_get))

(event EventTick
  (params (DeltaSeconds :type Float%20%28single-precision%29))
  ;[1 1 1] Tick Events
  (switch Utilities|FlowControl|Switch|SwitchonEWeapon_Ranged_Behaviors (Variables|Gameplay|GetFireMode)
    (:NewEnumerator0
      (CallFunction|TickSemiAuto))
    (:NewEnumerator1
      (CallFunction|TickFullAuto))
    (:NewEnumerator2
      (CallFunction|TickCharge))))

(event EventInputTriggerRelease
  ;[1 1 1] Trigger Events
  (Variables|Internal|SetIsInputTriggerPressed? false)
  (switch Utilities|FlowControl|Switch|SwitchonEWeapon_Ranged_Behaviors (Variables|Gameplay|GetFireMode)
    (:NewEnumerator0
      (CallFunction|ReleaseSemiAuto))
    (:NewEnumerator1
      (CallFunction|ReleaseFullAuto))
    (:NewEnumerator2
      (CallFunction|ReleaseCharge))))

(event EventInputTriggerPressed
  ;[1 1 1] Trigger Events
  (Variables|Internal|SetIsInputTriggerPressed? true)
  (switch Utilities|FlowControl|Switch|SwitchonEWeapon_Ranged_Behaviors (Variables|Gameplay|GetFireMode)
    (:NewEnumerator0
      (CallFunction|PressedSemiAuto))
    (:NewEnumerator1
      (CallFunction|PressedFullAuto))
    (:NewEnumerator2
      (CallFunction|PressedCharge))))

(fn ConstructionScript
  (|CallParentFunction))

(fn GetChargePercent
  (if (Utilities|Enum|Equal(Enum) (Variables|Gameplay|GetFireMode) "NewEnumerator2")
    (return (/ (Variables|Internal|GetCharge_ShotCharge) (Variables|Gameplay-Charge|GetCharge_FullChargeTime)))
    (else
      (return -1.0))))