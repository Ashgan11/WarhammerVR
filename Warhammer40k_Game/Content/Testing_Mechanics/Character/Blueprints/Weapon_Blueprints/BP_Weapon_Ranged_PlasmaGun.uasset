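; BP_Weapon_Ranged_PlasmaGun is a plasma gun weapon Blueprint that animates a charge-driven Mask component.
; Each tick, after running the parent logic, it eases ChargePercenCur toward ChargePercent with a fixed-alpha, frame-rate-dependent Lerp.
; The smoothed value is scaled and offset to set the Mask's relative Y position, so the mask slides with the charge level.
; The construction script only calls the parent.
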(event EventTick
  (params (DeltaSeconds :type Float%20%28single-precision%29))
  (bind _mask (Variables|Default|GetMask))
  (bind _relativelocation (Variables|/Script/Engine.SceneComponent|GetRelativeLocation _mask))
  (|CallParentFunction DeltaSeconds)
  (Variables|Internal|SetChargePercenCur (Math|Float|Lerp (Variables|Internal|GetChargePercenCur) (Variables|Default|GetChargePercent) 0.1))
  (Transformation|SetRelativeLocation _mask (Math|Vector|MakeVector (.x _relativelocation) (+ (* (* (Variables|Internal|GetChargePercenCur) 1e+02) 0.56) 4.5) (.z _relativelocation)) false false))

(fn ConstructionScript
  (|CallParentFunction))