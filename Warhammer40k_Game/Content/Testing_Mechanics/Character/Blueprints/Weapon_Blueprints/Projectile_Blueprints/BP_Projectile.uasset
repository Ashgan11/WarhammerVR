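; BP_Projectile is a weapon projectile actor that deals damage on impact.
; A timer set at BeginPlay destroys it after TimeToLive.
; A hit on ProjectileMesh applies point damage to whatever it struck, with no filtering of targets, crediting the instigator, then destroys the projectile after a short delay.
; The Collision overlap event is empty and an ApplyDamage call is left disconnected.
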(event OnComponentBeginOverlap(Collision)
  (params (OverlappedComponent :type Primitive%20Component%20Object%20Reference) (OtherActor :type Actor%20Object%20Reference) (OtherComp :type Primitive%20Component%20Object%20Reference) (OtherBodyIndex :type Integer) (bFromSweep :type Boolean) (SweepResult :type Hit%20Result%20Structure%20%28by%20ref%29)))

(event OnComponentHit(ProjectileMesh)
  (params (HitComponent :type Primitive%20Component%20Object%20Reference) (OtherActor :type Actor%20Object%20Reference) (OtherComp :type Primitive%20Component%20Object%20Reference) (NormalImpulse :type Vector :default "0, 0, 0") (Hit :type Hit%20Result%20Structure%20%28by%20ref%29))
  ;[1 1 1] Damage on collision (needs refinement, eg. check for a tag or cast to class to see if object should be damaged)
  (Game|Damage|ApplyPointDamage OtherActor (Variables|Gameplay|GetBase%20Damage) NormalImpulse Hit (Game|GetInstigatorController) (Game|GetInstigator) (Variables|Gameplay|GetDamage%20Type%20Class))
  (Utilities|FlowControl|Delay 0.33)
  ;[1 1 1] Set up self-destruct
  (Actor|DestroyActor))

(event Custom|Self-Destruct
  ;[1 1 1] Set up self-destruct
  (Actor|DestroyActor))

(event EventBeginPlay
  ;[1 1 1] Set up self-destruct
  (Utilities|Time|SetTimerbyEvent (delegate Custom|Self-Destruct) (Variables|Gameplay|GetTimeToLive)))

(fn ConstructionScript)