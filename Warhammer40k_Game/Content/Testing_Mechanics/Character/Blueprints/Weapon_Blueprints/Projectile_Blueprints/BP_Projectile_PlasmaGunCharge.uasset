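; Charged plasma gun projectile that acts as an instant beam, damaging enemies once when it spawns.
; On BeginPlay it sets the Niagara beam length, then runs a debug-drawn multi-sphere trace that ignores player pawns and applies point damage to BP_Enemy_Base hits.
; The trace end is the forward vector times BeamLength, without adding the actor's location.
; An unconnected branch setting beam start and end vectors never runs.
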(event EventBeginPlay
  (bind _returnvalue (Transformation|GetActorLocation))
  (bind _returnvalue_2 (Transformation|GetActorForwardVector))
  (bind _beam_length (Variables|Gameplay|GetBeam_Length))
  (bind _returnvalue_3 (* _returnvalue_2 _beam_length))
  (|CallParentFunction)
  (bind _outactors (Actor|GetAllActorsOfClass "/Game/Testing_Mechanics/Character/Blueprints/Character_Blueprints/BP_PlayerPawn.BP_PlayerPawn_C"))
  (Niagara|SetNiagaraVariable(Float) (Variables|Default|GetParticleSystem) "BeamLength" (Math|Vector|VectorLength (- _returnvalue_3 _returnvalue)))
  (bind (_outhits _returnvalue_4) (Collision|MultiSphereTraceByChannel _returnvalue _returnvalue_3 (Variables|Gameplay|GetBeam_Thickness) "TraceTypeQuery2" false _outactors "ForDuration"))
  (if _returnvalue_4
    (for _array_element _outhits
      (bind _asbp_enemy_base (Utilities|Casting|CastToBP_Enemy_Base (.HitActor (Collision|BreakHitResult _array_element))))
      (Game|Damage|ApplyPointDamage _asbp_enemy_base (Variables|Default|GetBase%20Damage) (.Normal (Collision|BreakHitResult _array_element)) _array_element (Game|GetInstigatorController) (Game|GetInstigator) (Variables|Default|GetDamage%20Type%20Class)))))

(event Collision|EventActorBeginOverlap
  (params (OtherActor :type Actor%20Object%20Reference))
  (|CallParentFunction OtherActor) ; This node is disabled and will not be called.\nDrag off pins to build functionality.
)

(event EventTick
  (params (DeltaSeconds :type Float%20%28single-precision%29))
  (|CallParentFunction DeltaSeconds) ; This node is disabled and will not be called.\nDrag off pins to build functionality.
)

(fn ConstructionScript
  (|CallParentFunction))