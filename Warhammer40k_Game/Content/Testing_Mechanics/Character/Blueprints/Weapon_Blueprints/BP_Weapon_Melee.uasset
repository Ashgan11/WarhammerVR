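; Melee weapon Blueprint that damages enemies with motion-driven swings and blocks when held in position.
; Tick derives velocity from a blade socket; overlaps count only above minimum speed and within cut/stab angles set by construction-script arrows.
; Normal hits build decaying charge; at maximum, hits deal multiplied damage for a short window before resetting.
; A looping timer enables block collision when slow and near side or overhead orientations.
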(event OnComponentBeginOverlap(WeaponModel)
  (params (OverlappedComponent :type Primitive%20Component%20Object%20Reference) (OtherActor :type Actor%20Object%20Reference) (OtherComp :type Primitive%20Component%20Object%20Reference) (OtherBodyIndex :type Integer) (bFromSweep :type Boolean) (SweepResult :type Hit%20Result%20Structure%20%28by%20ref%29))
  (bind _returnvalue (Actor|GetParentActor))
  (bind _damageamount (Variables|Default|GetDamageAmount))
  (bind _damagetype (Variables|Default|GetDamageType))
  ;[1 1 1] Weapon Hit
  (if (== (Utilities|GetClass OtherActor) "/Game/Testing_Mechanics/Game_AI/Blueprints/BP_Enemy_Base.BP_Enemy_Base_C")
    (bind _return (CallFunction|IsSwingFastEnough?))
    (bind _returnvalue_2 (CallFunction|IsSwingLegalAngle?))
    (if (and _returnvalue_2 _return)
      (if (== (Variables|Internal|GetCharge_Cur) (Variables|Gameplay|GetCharge_Max))
        (Game|Damage|ApplyDamage OtherActor (* _damageamount (Variables|Gameplay|GetCharge_DamageMultiplier)) 0 _returnvalue _damagetype) ; Charged Hit
        (Utilities|FlowControl|DoOnce false :!label _label
          (:Completed
            (Utilities|FlowControl|Delay (Variables|Gameplay|GetCharge_SwingSustain))
            (Variables|Internal|SetCharge_Cur 0.0)
            (goto _label Reset)))
        (else
          (CallFunction|ChargeAdd 1.0 true) ; 1 Charge for normal hit
          (Game|Damage|ApplyDamage OtherActor _damageamount 0 _returnvalue _damagetype) ; Uncharged Hit
        )))))

(event Custom|Validate%20Blocking%20Stance
  (bind _weaponmodel (Variables|Default|GetWeaponModel))
  (bind _weaponmodel_2 (Variables|Default|GetWeaponModel))
  (bind _returnvalue (Transformation|GetWorldRotation _weaponmodel))
  (bind _returnvalue_2 (Transformation|GetWorldRotation _weaponmodel_2))
  (bind (_roll _pitch) (Math|Rotator|BreakRotator _returnvalue_2))
  (bind (_roll_2 _pitch_2) (Math|Rotator|BreakRotator _returnvalue))
  ;[1 1 1] Periodically check if sword is held in viable blocking orientation.
  (bind _return (CallFunction|IsSwingFastEnough?))
  (CallFunction|ToggleBlockCollision (and (not _return) (or (Math|Rotator|Equal(Rotator) (Variables|Gameplay|GetDesiredBlockOrientation_Side) (Math|Rotator|MakeRotator _roll_2 _pitch_2 0.0) (Variables|Gameplay|GetDesiredBlockOrientationTolerance)) (Math|Rotator|Equal(Rotator) (Variables|Gameplay|GetDesiredBlockOrientation_Overhead) (Math|Rotator|MakeRotator _roll _pitch 0.0) (Variables|Gameplay|GetDesiredBlockOrientationTolerance))))))

(event Custom|Charge%20Add
  (params (Delta%20Charge :type Float%20%28single-precision%29) (ResetTimer? :type Boolean))
  ;[1 1 1] Modify charges
  (Variables|Internal|SetCharge_Cur (Math|Float|Clamp(Float) (+ Delta%20Charge (Variables|Internal|GetCharge_Cur)) 0.0 (Variables|Gameplay|GetCharge_Max)))
  (if ResetTimer?
    (Variables|Internal|SetCharge_DecayTimer 0.0)))

(event Custom|Charge%20Decay
  ;[1 1 1] Increment decay timer & remove charges if decay is active
  (bind _output_get (Variables|Internal|SetCharge_DecayTimer (Math|Float|Clamp(Float) (+ (Variables|Internal|GetCharge_DecayTimer) (Utilities|Time|GetWorldDeltaSeconds)) 0.0 (Variables|Gameplay|GetCharge_DecayStart))))
  (Math|Float|CompareFloat _output_get (Variables|Gameplay|GetCharge_DecayStart)
    (:>
      _)
    (:==
      _))
  (CallFunction|ChargeAdd (* (Variables|Gameplay|GetCharge_DecayRate) (Utilities|Time|GetWorldDeltaSeconds) -1.0) false))

(event EventBeginPlay
  ;[1 1 1] Initialize
  (Variables|Internal|SetLastSocketPosition (Transformation|GetSocketLocation (Variables|Default|GetWeaponModel) "Middle"))
  (CallFunction|ToggleBlockCollision false)
  (Utilities|Time|SetTimerbyEvent (delegate Custom|Validate%20Blocking%20Stance) 0.1 true))

(event EventTick
  (params (DeltaSeconds :type Float%20%28single-precision%29))
  (bind _weaponmodel (Variables|Default|GetWeaponModel))
  (bind _returnvalue (Transformation|GetSocketLocation _weaponmodel "Middle"))
  ;[1 1 1] Tick. Handles updating current and previous socket position for now.
  (Variables|Internal|SetVelocityCur (- _returnvalue (Variables|Internal|GetLastSocketPosition)))
  (Variables|Internal|SetLastSocketPosition _returnvalue)
  (bind _returnvalue_2 (CallFunction|GetChargePercent))
  (Variables|Internal|SetCharge_PercentCur _returnvalue_2)
  (CallFunction|ChargeDecay))

(fn ConstructionScript
  (bind _angle_cut (Variables|Gameplay|GetAngle_Cut))
  (bind _angle_stab (Variables|Gameplay|GetAngle_Stab))
  (bind _returnvalue (/ _angle_stab 2.0))
  (bind _returnvalue_2 (/ _angle_cut 2.0))
  (|CallParentFunction)
  (Utilities|FlowControl|Sequence
    (:then_0
      (Transformation|SetRelativeRotation (Variables|Default|GetArrow_Cut_Min) (Math|Rotator|MakeRotator 0.0 0.0 (* _returnvalue_2 -1.0)) false false)
      (Transformation|SetRelativeRotation (Variables|Default|GetArrow_Cut_Max) (Math|Rotator|MakeRotator 0.0 0.0 _returnvalue_2) false false))
    (:then_1
      (Transformation|SetRelativeRotation (Variables|Default|GetArrow_Stab_Min) (Math|Rotator|MakeRotator 0.0 0.0 (* _returnvalue -1.0)) false false)
      (Transformation|SetRelativeRotation (Variables|Default|GetArrow_Stab_Max) (Math|Rotator|MakeRotator 0.0 0.0 _returnvalue) false false))))

(fn IsSwingFastEnough?
  (Math|Float|CompareFloat (Math|Vector|VectorLength (Variables|Internal|GetVelocityCur)) (Variables|Gameplay|GetVelocityMin)
    (:>
      _)
    (:==
      _)
    (:<
      (return false)))
  (return true))

(fn IsSwingLegalAngle?
  (bind _weaponmodel (Variables|Default|GetWeaponModel))
  (bind _angle_cut (Variables|Gameplay|GetAngle_Cut))
  (bind _lastsocketposition (Variables|Internal|GetLastSocketPosition))
  (bind _angle_stab (Variables|Gameplay|GetAngle_Stab))
  (bind _returnvalue (Transformation|GetSocketLocation _weaponmodel "Middle"))
  (bind _returnvalue_2 (+ _angle_cut _angle_stab))
  (bind _returnvalue_3 (/ _returnvalue_2 4.0))
  (bind _returnvalue_4 (Math|Vector|GetUnitDirection(Vector) _lastsocketposition _returnvalue))
  (bind _returnvalue_5 (+ _returnvalue_3 1.4e+02 0.01))
  ;[1 0 0.104] Calculating Angles and comparing them to max Angle / Calculating hit angle
  (return (Math|Boolean|NORBoolean (> (+ (Class|KismetMathLibrary|DegAcos (Math|Vector|DotProduct (Math|Vector|GetForwardVector (Variables|Default|GetArrow_Stab_Max)) _returnvalue_4)) (Class|KismetMathLibrary|DegAcos (Math|Vector|DotProduct (Math|Vector|GetForwardVector (Variables|Default|GetArrow_Cut_Min)) _returnvalue_4))) _returnvalue_5) (> (+ (Class|KismetMathLibrary|DegAcos (Math|Vector|DotProduct (Math|Vector|GetForwardVector (Variables|Default|GetArrow_Stab_Min)) _returnvalue_4)) (Class|KismetMathLibrary|DegAcos (Math|Vector|DotProduct (Math|Vector|GetForwardVector (Variables|Default|GetArrow_Cut_Max)) _returnvalue_4))) _returnvalue_5))))

(fn ToggleBlockCollision
  (params (Blocking%20Active? :type Boolean))
  (bind _collision_hardblock (Variables|Default|GetCollision_HardBlock))
  (bind _collision_softblock (Variables|Default|GetCollision_SoftBlock))
  (if Blocking%20Active?
    (Collision|SetCollisionEnabled _collision_hardblock "QueryOnly")
    (Collision|SetCollisionEnabled _collision_softblock "QueryOnly")
    (else
      (Collision|SetCollisionEnabled _collision_hardblock "NoCollision")
      (Collision|SetCollisionEnabled _collision_softblock "NoCollision"))))

(fn GetChargePercent
  (return (/ (Variables|Internal|GetCharge_Cur) (Variables|Gameplay|GetCharge_Max))))