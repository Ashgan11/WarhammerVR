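; BP_Weapon_Melee is a melee weapon prototype that tests whether the blade moves within an allowed hit angle.
; Each Tick, it derives the movement direction of the "Middle" socket from its previous position.
; Dot-product angles to four arrow components are summed in two pairs, and it prints true only if neither sum exceeds a fixed limit.
; An unconnected Rotate timeline holds test motion for the weapon model.
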(event EventBeginPlay
  ;[1 0 0.104] Calculating Angles and comparing them to max Angle / Calculating hit angle
  (Variables|Default|SettestVectorMiddle (Transformation|GetSocketLocation (Variables|Default|GetWeaponModel) "Middle")))

(event EventTick
  (params (DeltaSeconds :type Float%20%28single-precision%29))
  (bind _arrow (Variables|Default|GetArrow))
  (bind _arrow1 (Variables|Default|GetArrow1))
  (bind _arrow2 (Variables|Default|GetArrow2))
  (bind _arrow3 (Variables|Default|GetArrow3))
  (bind _returnvalue (Math|Vector|GetForwardVector _arrow))
  (bind _returnvalue_2 (Math|Vector|GetForwardVector _arrow1))
  (bind _returnvalue_3 (Math|Vector|GetForwardVector _arrow2))
  (bind _returnvalue_4 (Math|Vector|GetForwardVector _arrow3))
  ;[1 0 0.104] Calculating Angles and comparing them to max Angle / Calculating hit angle
  (Development|PrintString (Utilities|String|ToString(Boolean) (Math|Boolean|NORBoolean (> (+ (Class|KismetMathLibrary|DegAcos (/ (Math|Vector|DotProduct _returnvalue (Math|Vector|GetUnitDirection(Vector) (Variables|Default|GettestVectorMiddle) (Transformation|GetSocketLocation (Variables|Default|GetWeaponModel) "Middle"))) (* (Math|Vector|VectorLength _returnvalue) (Math|Vector|VectorLength (Math|Vector|GetUnitDirection(Vector) (Variables|Default|GettestVectorMiddle) (Transformation|GetSocketLocation (Variables|Default|GetWeaponModel) "Middle")))))) (Class|KismetMathLibrary|DegAcos (/ (Math|Vector|DotProduct _returnvalue_4 (Math|Vector|GetUnitDirection(Vector) (Variables|Default|GettestVectorMiddle) (Transformation|GetSocketLocation (Variables|Default|GetWeaponModel) "Middle"))) (* (Math|Vector|VectorLength _returnvalue_4) (Math|Vector|VectorLength (Math|Vector|GetUnitDirection(Vector) (Variables|Default|GettestVectorMiddle) (Transformation|GetSocketLocation (Variables|Default|GetWeaponModel) "Middle"))))))) 1e+02) (> (+ (Class|KismetMathLibrary|DegAcos (/ (Math|Vector|DotProduct _returnvalue_2 (Math|Vector|GetUnitDirection(Vector) (Variables|Default|GettestVectorMiddle) (Transformation|GetSocketLocation (Variables|Default|GetWeaponModel) "Middle"))) (* (Math|Vector|VectorLength _returnvalue_2) (Math|Vector|VectorLength (Math|Vector|GetUnitDirection(Vector) (Variables|Default|GettestVectorMiddle) (Transformation|GetSocketLocation (Variables|Default|GetWeaponModel) "Middle")))))) (Class|KismetMathLibrary|DegAcos (/ (Math|Vector|DotProduct _returnvalue_3 (Math|Vector|GetUnitDirection(Vector) (Variables|Default|GettestVectorMiddle) (Transformation|GetSocketLocation (Variables|Default|GetWeaponModel) "Middle"))) (* (Math|Vector|VectorLength _returnvalue_3) (Math|Vector|VectorLength (Math|Vector|GetUnitDirection(Vector) (Variables|Default|GettestVectorMiddle) (Transformation|GetSocketLocation (Variables|Default|GetWeaponModel) "Middle"))))))) 1e+02))))
  (Variables|Default|SettestVectorMiddle (Transformation|GetSocketLocation (Variables|Default|GetWeaponModel) "Middle")))

(fn ConstructionScript
  (|CallParentFunction))